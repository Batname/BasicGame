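; MyPlayer_BP is the player Blueprint that sets up the on-screen HUD and a crosshair mouse cursor.
; BeginPlay creates and stores the HUD widget, adds it to the viewport, configures the player controller's cursor and makes the arrow component visible in game.
; The HUDUpdateHP event forwards health refreshes to the widget.
; Logic to yaw the actor toward the deprojected mouse position exists but is unconnected, and Tick is empty.
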(event EventBeginPlay
  (bind _returnvalue (UserInterface|CreateWidget "/Game/Blueprints/HUD.HUD_C"))
  (bind _output_get (Variables|Default|SetHUD _returnvalue))
  (UserInterface|Viewport|AddtoViewport _output_get 0)
  (bind _asplayer_controller (Utilities|Casting|CastToPlayerController (Pawn|GetController)))
  (Variables|/Script/Engine.PlayerController|SetbShowMouseCursor _asplayer_controller true)
  (Variables|/Script/Engine.PlayerController|SetCurrentMouseCursor _asplayer_controller "Crosshairs")
  (Development|SetHiddeninGame (Variables|Default|GetArrowComponent) false false))

(event Collision|EventActorBeginOverlap
  (params (OtherActor :type Actor%20Object%20Reference)))

(event EventHUDUpdateHP
  (Default|UpdateHealth (Variables|Default|GetHUD)))

(event EventTick
  (params (DeltaSeconds :type Float%20%28single-precision%29)))

(fn ConstructionScript)